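; BP_GoldOre is a gold loot pickup that launches as a projectile and is collected on overlap.
; Construction picks one of three gold meshes at random and applies the exposed initial speed to the projectile movement.
; On hit, it stops projectile movement and hands the mesh over to physics simulation.
; The first overlapping actor implementing BPI_Loot receives a fixed-value loot message, then the ore destroys itself.
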(event `self.ReceiveHit`
  (params (MyComp :type "PrimitiveComponent Object Reference") (Other :type "Actor Object Reference") (OtherComp :type "PrimitiveComponent Object Reference") (bSelfMoved :type Boolean) (HitLocation :type "Vector Structure") (HitNormal :type "Vector Structure") (NormalImpulse :type "Vector Structure") (Hit :type "HitResult Structure (by ref)"))
  (`ActorComponent.Deactivate` (`self.ProjectileMovement`))
  (`PrimitiveComponent.SetSimulatePhysics` (`self.StaticMesh`) true))

(event `self.ReceiveActorBeginOverlap`
  (params (OtherActor :type "Actor Object Reference"))
  (if (`KismetSystemLibrary.DoesImplementInterface` OtherActor "/Game/Blueprints/Loot/BPI_Loot.BPI_Loot_C")
    (`/Engine/EditorBlueprintResources/StandardMacros.DoOnce` false
      (:`Completed`
        (message `/Game/Blueprints/Loot/BPI_Loot.Receive Loot` OtherActor 5.0)
        (`self.K2_DestroyActor`)))))

(fn `UserConstructionScript`
  (`StaticMeshComponent.SetStaticMesh` (`self.StaticMesh`) (select `int` (`KismetMathLibrary.RandomInteger` 3) :`0` "/Game/Meshes/SM_Gold_01.SM_Gold_01" :`1` "/Game/Meshes/SM_Gold_02.SM_Gold_02" :`2` "/Game/Meshes/SM_Gold_03.SM_Gold_03" :!type "StaticMesh Object Reference"))
  (set `ProjectileMovementComponent.InitialSpeed` (`self.Initial Speed`) (`self.ProjectileMovement`)))