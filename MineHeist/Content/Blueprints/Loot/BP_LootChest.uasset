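; BP_LootChest is a loot chest that hands out loot to whoever vacuums it.
; On BeginPlay it binds its RotatingMovement component to the Wheel.
; Each Vacuumed event sends a placeholder loot amount to the Perpetrator and plays the Vacuuming sequence if it is not already playing.
; A DoOnce reset after a Frequency delay throttles how often loot is given.
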(event `self.ReceiveBeginPlay`
  (`self.Init Wheel`))

(event `/Game/Blueprints/PlayerPawn/BPI_Vaccuumable.Vacuumed`
  (params (Perpetrator :type "Actor Object Reference"))
  (bind _sequenceplayer (`ActorSequenceComponent.SequencePlayer` (`self.Vacuuming`)))
  (`/Engine/EditorBlueprintResources/StandardMacros.DoOnce` false :!label _label
    (:`Completed`
      (message `/Game/Blueprints/Loot/BPI_Loot.Receive Loot` Perpetrator (`self.Placeholder Loot Amount`))
      (if (not (`MovieSceneSequencePlayer.IsPlaying` _sequenceplayer))
        (`MovieSceneSequencePlayer.Play` _sequenceplayer))
      (`KismetSystemLibrary.Delay` (`self.Frequency`))
      (goto _label :!via `Reset`))))

(fn `Init Wheel`
  (`MovementComponent.SetUpdatedComponent` (`self.RotatingMovement`) (`self.Wheel`)))

(fn `UserConstructionScript`)