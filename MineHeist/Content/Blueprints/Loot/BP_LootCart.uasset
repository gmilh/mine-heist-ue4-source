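; Per-player loot cart that tallies collected ore toward a target fetched from the game mode.
; Loot adds to the total, fires LootIncreased with the player index, plays a sound and unhides Ore child meshes in proportion to progress toward the target.
; PlayerIndex picks one of four colours, applied to the point light at construction and to the cart and lid through a dynamic material instance.
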(event EventBeginPlay
  (bind _target (Class|BPIGameMode|GetTargetLoot(Message) (Game|GetGameMode)))
  (Variables|Default|SetTarget%20Loot _target)
  (Utilities|FlowControl|Delay 0.2)
  (CallFunction|InitColour))

(event EventLoot
  (params (Amount :type Float%20%28single-precision%29))
  (bind _ores (Variables|Default|GetOres))
  (bind _children (Components|GetChildrenComponents _ores false))
  (bind _output_get (Variables|Default|SetLoot%20Collected (+ Amount (Variables|Default|GetLoot%20Collected))))
  (Default|CallLootIncreased _output_get (Variables|Default|GetPlayer%20Index))
  (Audio|SpawnSoundatLocation "/Game/Audio/SFX/SC_GainedOre.SC_GainedOre" "0, 0, 0" "0, 0, 0" 1.0 0.4 0.0 0 0)
  (for _index (range 0 (|((Length*Current)/Target) (Utilities|Array|Length _children) (Math|Float|Truncate (Variables|Default|GetLoot%20Collected)) (Variables|Default|GetTarget%20Loot)))
    (Development|SetHiddeninGame (Utilities|Array|Get(acopy) _children _index) false false)))

(fn ConstructionScript
  (CallFunction|InitColour)
  (Rendering|Components|Light|SetLightColor (Variables|Default|GetPointLight) (Utilities|Select :Index (Variables|Default|GetPlayer%20Index) :Option%200 "(R=1.000000,G=0.829889,B=0.263283,A=1.000000)" :Option%201 "(R=0.000000,G=0.569136,B=1.000000,A=1.000000)" :Option%202 "(R=1.000000,G=0.000000,B=0.047706,A=1.000000)" :Option%203 "(R=0.000000,G=1.000000,B=0.020782,A=1.000000)") true))

(fn InitColour
  (bind _returnvalue (Rendering|Material|CreateDynamicMaterialInstance (Variables|Default|GetStaticMesh) 0 "/Game/Materials/MI_Backpack.MI_Backpack" "None" :!class /Script/Engine.PrimitiveComponent))
  (bind _output_get (LocalVariables|SetPlayer%20Colour%20Material _returnvalue))
  (Rendering|Material|SetVectorParameterValue _output_get "Colour" (Utilities|Select :Index (Variables|Default|GetPlayer%20Index) :Option%200 "(R=1.000000,G=0.829889,B=0.263283,A=1.000000)" :Option%201 "(R=0.000000,G=0.569136,B=1.000000,A=1.000000)" :Option%202 "(R=1.000000,G=0.000000,B=0.047706,A=1.000000)" :Option%203 "(R=0.000000,G=1.000000,B=0.020782,A=1.000000)") :!class /Script/Engine.MaterialInstanceDynamic)
  (Rendering|Material|SetMaterial (Variables|Default|GetStaticMesh) 0 (LocalVariables|GetPlayer%20Colour%20Material))
  (Rendering|Material|SetMaterial (Variables|Default|GetStaticMesh) 2 (LocalVariables|GetPlayer%20Colour%20Material)))