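; BP_SmallObject_Base is a base Blueprint for small objects that react to being vacuumed.
; Its Vacuumed event pulls the static mesh toward the perpetrator with a mass-independent force, built from a normalized direction, a strength and an offset.
; Each call also makes a loud noise at the object's location through a PawnNoiseEmitter, which pawn-sensing listeners can hear.
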(event `/Game/Blueprints/PlayerPawn/BPI_Vaccuumable.Vacuumed`
  (params (Perpetrator :type "Actor Object Reference"))
  (`PrimitiveComponent.AddForce` (`self.StaticMesh`) (+ (* (`KismetMathLibrary.Normal` (- (`self.K2_GetActorLocation` Perpetrator) (`self.K2_GetActorLocation`))) (`self.Vacuuming Push Strength`)) (`self.Vacuuming Push Offset`)) "None" true)
  (`PawnNoiseEmitterComponent.MakeNoise` (`self.PawnNoiseEmitter`) self 2000.0 (`self.K2_GetActorLocation` self)))

(fn `UserConstructionScript`)