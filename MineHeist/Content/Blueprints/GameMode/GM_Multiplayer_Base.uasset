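; Base game mode for local multiplayer that creates three additional local players and spawns each at its own start point when a lift signals ready.
; BeginPlay creates the players, then sets BP_PlayerCharacter as the default pawn and binds to every BP_Lift's ready event.
; That event's index selects a player controller, which is restarted at the PlayerStart whose tag matches its controller ID.
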(event `self.ReceiveBeginPlay`
  (`GameplayStatics.CreatePlayer` -1)
  (`GameplayStatics.CreatePlayer` -1)
  (`GameplayStatics.CreatePlayer` -1)
  (`parent.ReceiveBeginPlay`)
  (set `self.DefaultPawnClass` "/Game/Blueprints/PlayerPawn/BP_PlayerCharacter.BP_PlayerCharacter_C")
  (bind _outactors (`GameplayStatics.GetAllActorsOfClass` "/Game/Blueprints/GameMode/BP_Lift.BP_Lift_C"))
  (for _array_element _outactors
    (add `/Game/Blueprints/GameMode/BP_Lift.Lift Ready` _array_element (delegate `Handle Lift Ready`))))

(event `Handle Lift Ready`
  (params (Index :type Integer))
  (bind _returnvalue (`GameplayStatics.GetPlayerController` Index))
  (`self.RestartPlayerAtPlayerStart` _returnvalue (`self.Get Start Spot by Player Index` _returnvalue)))

(fn `Get Start Spot by Player Index`
  (params (Player :type "PlayerController Object Reference"))
  (returns (`Array Element` :type "PlayerStart Object Reference"))
  (bind _outactors (`GameplayStatics.GetAllActorsOfClass` "/Script/Engine.PlayerStart"))
  (for _array_element _outactors
    (if (== (`KismetStringLibrary.Conv_StringToName` (`KismetStringLibrary.Conv_IntToString` (`GameplayStatics.GetPlayerControllerID` Player))) (`PlayerStart.PlayerStartTag` _array_element))
      (return _array_element))))

(fn `UserConstructionScript`
  (`parent.UserConstructionScript`))