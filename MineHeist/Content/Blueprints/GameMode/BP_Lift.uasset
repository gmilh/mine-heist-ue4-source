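; Per-player lift actor that bundles a player start and a loot cart for the player given by its PlayerIndex.
; The construction script tags the child PlayerStart with that index, and BeginPlay copies it to the child BP_LootCart.
; DeployLift starts an eased move of the Lift component over DescendLength, then fires LiftReady with the index and hides the light.
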(event `self.ReceiveBeginPlay`
  (`self.Init Chest Colour`))

(event `/Game/Blueprints/GameMode/BPI_Lift.Deploy Lift`
  (`KismetSystemLibrary.MoveComponentTo` (`self.Lift`) (0.0 0.0 0.0) (struct :`Yaw` -90.0) false true (`self.Descend length`))
  (`self.Lift Ready` (`self.Player Index`))
  (`self.SetActorHiddenInGame` (`self.Light`) true))

(fn `Check Index`
  (returns (`Player Index` :type Integer))
  (return (`self.Player Index`)))

(fn `Init Chest Colour`
  (bind _asbp_loot_cart (cast `/Game/Blueprints/Loot/BP_LootCart` (`ChildActorComponent.ChildActor` (`self.Chest`)))
    (:`then`
      (set `/Game/Blueprints/Loot/BP_LootCart.Player Index` (`self.Player Index`) _asbp_loot_cart))
    (:`CastFailed`
      (`KismetSystemLibrary.PrintString` "Hello"))))

(fn `Init Starter`
  (bind _asplayer_start (cast `PlayerStart` (`ChildActorComponent.ChildActor` (`self.Start`))))
  (set `PlayerStart.PlayerStartTag` (`KismetStringLibrary.Conv_StringToName` (`KismetStringLibrary.Conv_IntToString` (`self.Player Index`))) _asplayer_start))

(fn `UserConstructionScript`
  (`self.Init Starter`))