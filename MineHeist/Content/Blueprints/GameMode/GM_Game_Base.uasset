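; Base game mode for a timed loot-collection game, with win and time-expired messages sent to the HUD.
; On BeginPlay it finds or spawns the camera, starts the session timer, binds to loot carts and starts music.
; Reaching the target loot clears the timer and declares the win.
; Enemy alert events maintain a set of active notifiers, fading alert music in while any remain and pausing the background track.
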(event `self.ReceiveBeginPlay`
  (`self.Init Camera`)
  (`self.Init Timer`)
  (`self.Init Loot Collection Notifiers`)
  (`self.Init Music`))

(event `Register Alert`
  (params (`Notifier ID` :type String))
  ;[1 1 1] Update Registered Alerts
  (`KismetArrayLibrary.Array_AddUnique` (`self.Active Alerts`) `Notifier ID`)
  (`self.Update Music`))

(event `Initiate Alert Music`
  (bind _fade_in_alert (`self.Fade In Alert`))
  ;[1 1 1] Transition to and from Alert Music
  (if (not (`AudioComponent.IsPlaying` (`self.SC_AlertMusic`)))
    (`AudioComponent.FadeIn` (`self.SC_AlertMusic`) _fade_in_alert 1.0 0.0)
    (`KismetSystemLibrary.Delay` _fade_in_alert)
    (`AudioComponent.SetPaused` (`self.SC_BackgroundMusic`) true)))

(event `Clear Alert`
  (params (`Notifier ID` :type String))
  ;[1 1 1] Update Registered Alerts
  (`KismetArrayLibrary.Array_RemoveItem` (`self.Active Alerts`) `Notifier ID`)
  (`self.Update Music`))

(event `End Alert Music`
  ;[1 1 1] Transition to and from Alert Music
  (if (`AudioComponent.IsPlaying` (`self.SC_AlertMusic`))
    (`AudioComponent.SetPaused` (`self.SC_BackgroundMusic`) false)
    (`AudioComponent.FadeOut` (`self.SC_AlertMusic`) (`self.Fade Out Alert`) 0.0)))

(fn `Abort Timer`
  (`KismetSystemLibrary.K2_ClearAndInvalidateTimerHandle` (`self.Session Timer`)))

(fn `Get Target Loot`
  (returns (Target :type Integer))
  (return (`self.Target Loot`)))

(fn `Handle Loot Collected`
  (params (`New Amount` :type "Float (double-precision)") (ID :type Integer))
  (if (>= `New Amount` (`KismetMathLibrary.Conv_IntToDouble` (`self.Target Loot`)))
    (`self.Abort Timer`)
    (`self.Loot Reached` ID)))

(fn `Init Camera`
  (bind _returnvalue (`GameplayStatics.GetPlayerController` 0))
  (bind _outactors (`GameplayStatics.GetAllActorsOfClass` "/Game/Blueprints/Camera/BP_Camera_Base.BP_Camera_Base_C"))
  (if (`KismetArrayLibrary.Array_IsValidIndex` _outactors)
    (set `self.Game Camera` (`|GetArrayItem` _outactors))
    (else
      (bind _returnvalue_2 (`|SpawnActorFromClass` (`self.Camera Class`) (`self.GetTransform` (`self.K2_FindPlayerStart` _returnvalue)) "Undefined" "OverrideRootScale" _returnvalue null))
      (set `self.Game Camera` _returnvalue_2))))

(fn `Init Loot Collection Notifiers`
  (bind _outactors (`GameplayStatics.GetAllActorsOfClass` "/Game/Blueprints/Loot/BP_LootCart.BP_LootCart_C"))
  (for _array_element _outactors
    (add `/Game/Blueprints/Loot/BP_LootCart.Loot Increased` _array_element (`|CreateDelegate` :!event `Handle Loot Collected`))))

(fn `Init Music`
  (`AudioComponent.Play` (`self.SC_BackgroundMusic`) 0.0)
  (`GameplayStatics.PlaySoundAtLocation` "/Game/Audio/SFX/SC_Ambiance.SC_Ambiance" (0.0 0.0 0.0) (struct) 1.0 1.0 0.0 null null null)
  ;[1 1 1] Setup Alert Music Changes
  (bind _outactors (`GameplayStatics.GetAllActorsOfClass` "/Game/Blueprints/AI/BP_EnemyPawn_Base.BP_EnemyPawn_Base_C"))
  (for _array_element _outactors
    (add `/Game/Blueprints/AI/BP_EnemyPawn_Base.On Alert` _array_element (`|CreateDelegate` :!event `Register Alert`))
    (add `/Game/Blueprints/AI/BP_EnemyPawn_Base.All Clear` _array_element (`|CreateDelegate` :!event `Clear Alert`))))

(fn `Init Timer`
  (bind _returnvalue (`KismetSystemLibrary.K2_SetTimer` self "Time Expired" (`self.Time Limit`)))
  (set `self.Session Timer` _returnvalue))

(fn `Loot Reached`
  (params (ID :type Integer))
  (message `/Game/Blueprints/UI/BPI_HUD.GameWin` (`PlayerController.GetHUD` (`GameplayStatics.GetPlayerController` 0)) ID)
  (`KismetSystemLibrary.K2_ClearAndInvalidateTimerHandle` (`self.Session Timer`)))

(fn `Time Expired`
  (message `/Game/Blueprints/UI/BPI_HUD.TimeExpired` (`PlayerController.GetHUD` (`GameplayStatics.GetPlayerController` 0))))

(fn `Update Music`
  (if (`KismetArrayLibrary.Array_IsValidIndex` (`self.Active Alerts`))
    (`self.Initiate Alert Music`)
    (else
      (`self.End Alert Music`))))

(fn `UserConstructionScript`
  (`parent.UserConstructionScript`))