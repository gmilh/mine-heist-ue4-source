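; BP_Camera_Base is a shared camera actor that follows the group of player-controlled pawns.
; On BeginPlay it caches the pawn of every PlayerController.
; When DynamicMovement is enabled, each Tick interpolates its location toward the pawns' average position plus CameraOffset at CameraSpeed.
; Rotation is set to a fixed downward angle, leaving an interpolated look-at rotation with CameraAngleOffset unused.
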(event `self.ReceiveBeginPlay`
  (`self.Store Player Pawn Refs`))

(event `self.ReceiveTick`
  (params (DeltaSeconds :type "Float (single-precision)"))
  (if (`self.Dynamic Movement`)
    (`self.Update Camera Location with Rotation`)))

(fn `Store Player Pawn Refs`
  (bind _outactors (`GameplayStatics.GetAllActorsOfClass` "/Script/Engine.PlayerController"))
  (for _array_element _outactors
    (`KismetArrayLibrary.Array_Add` (`self.Player Pawns`) (`Controller.K2_GetPawn` _array_element))))

(fn `Update Camera Location with Rotation`
  (bind _returnvalue (`GameplayStatics.GetActorArrayAverageLocation` (`self.Player Pawns`)))
  (`self.K2_SetActorLocationAndRotation` (`KismetMathLibrary.VInterpTo` (`self.K2_GetActorLocation`) (+ _returnvalue (`self.Camera Offset`)) (`GameplayStatics.GetWorldDeltaSeconds`) (`self.Camera Speed`)) (struct :`Pitch` -55.0) false true))

(fn `UserConstructionScript`)