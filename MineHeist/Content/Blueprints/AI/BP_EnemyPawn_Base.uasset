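; Base enemy AI pawn that walks a looping list of patrol points, switches between Patrol and Chase, and attacks with a pickaxe swing.
; State changes set walk speed, scale walk-animation rate, recolor a rect light and send alert or all-clear notifications.
; Sequence players drive walking and swinging.
; Whacks damage players already in the hitbox, then open a gate damaging new overlaps once each until the attack task finishes.
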(event OnComponentBeginOverlap(WhackingHitbox)
  (params (OverlappedComponent :type Primitive%20Component%20Object%20Reference) (OtherActor :type Actor%20Object%20Reference) (OtherComp :type Primitive%20Component%20Object%20Reference) (OtherBodyIndex :type Integer) (bFromSweep :type Boolean) (SweepResult :type Hit%20Result%20Structure%20%28by%20ref%29))
  (Utilities|FlowControl|Gate true
    (:Exit
      (if (not (Utilities|Array|ContainsItem (Variables|Default|GetWhacked) OtherActor))
        (if (Utilities|Array|IsValidIndex (Variables|Default|GetWhacked))
          _
          (else
            (Audio|PlaySoundatLocation "/Game/Audio/SFX/SC_AxedHit.SC_AxedHit" (Transformation|GetActorLocation OtherActor) "0, 0, 0" 1.0 1.0 0.0 0 0 0)))
        (Utilities|FlowControl|Sequence
          (:then_0
            (Game|Damage|ApplyDamage OtherActor (Variables|Default|GetWhack%20Damaged) (Pawn|GetController) self))
          (:then_1
            (Utilities|Array|Add (Variables|Default|GetWhacked) OtherActor)))))))

(event Custom|Set%20Gate%20Open
  (params (Open :type Boolean))
  (if Open
    (Utilities|FlowControl|Gate true) ; enters at Open
    (else
      (Utilities|FlowControl|Gate true) ; enters at Close
    )))

(event Custom|End%20Whacking
  (AI|BehaviorTree|FinishExecute (stale EventPerformWhacking Task%20Ref) true)
  (CallFunction|SetGateOpen false))

(event EventTick
  (params (DeltaSeconds :type Float%20%28single-precision%29))
  (if (Math|Vector|NotEqual(Vector) (Pawn|Components|CharacterMovement|GetLastUpdateVelocity (Variables|Character|GetCharacterMovement)) "0, 0, 0" 0.1)
    (if (not (Audio|Components|Audio|IsPlaying (Variables|/Script/ActorSequence.ActorSequenceComponent|GetSequencePlayer (Variables|Default|GetWalking))))
      (Class|MovieSceneSequencePlayer|PlayLooping (Variables|/Script/ActorSequence.ActorSequenceComponent|GetSequencePlayer (Variables|Default|GetWalking)) -1))
    (elif (Audio|Components|Audio|IsPlaying (Variables|/Script/ActorSequence.ActorSequenceComponent|GetSequencePlayer (Variables|Default|GetWalking)))
      (Class|MovieSceneSequencePlayer|GotoEndandStop (Variables|/Script/ActorSequence.ActorSequenceComponent|GetSequencePlayer (Variables|Default|GetWalking))))))

(event EventSetState
  (params (New%20State :type E_MinerStates%20Enum :default "NewEnumerator0"))
  (CallFunction|StatusChangeMovement New%20State)
  (CallFunction|StatusChangeVFX New%20State)
  (CallFunction|AlertStatusChangeNotifier New%20State))

(event EventPerformWhacking
  (params (Task%20Ref :type BT%20Task%20Blueprint%20Base%20Object%20Reference))
  (bind _pickaxe_swing (Variables|Default|GetPickaxe%20Swing))
  (bind _sequenceplayer (Variables|/Script/ActorSequence.ActorSequenceComponent|GetSequencePlayer _pickaxe_swing))
  (Sequencer|Player|Play _sequenceplayer :!class /Script/MovieScene.MovieSceneSequencePlayer)
  (EventDispatchers|BindEventtoOnFinished _sequenceplayer (EventDispatchers|CreateEvent :!event Custom|End%20Whacking)))

(fn ConstructionScript
  (Variables|/Script/Engine.CharacterMovementComponent|SetMaxWalkSpeed (Variables|Character|GetCharacterMovement) (.Value (Utilities|Map|Find (Variables|Default|GetSpeed) ""))))

(fn ExecuteWhacking
  (Audio|Components|Audio|Play (Variables|Default|GetSwing%20Sound) 0.0)
  (bind _output_get (Variables|Default|SetWhacked (Collision|GetOverlappingActors (Variables|Default|GetWhacking%20Hitbox) "/Game/Blueprints/PlayerPawn/BP_PlayerCharacter.BP_PlayerCharacter_C" :!class /Script/Engine.PrimitiveComponent)))
  (Development|PrintString (Utilities|String|ToString(Integer) (Utilities|Array|Length _output_get)))
  (if (Utilities|Array|IsValidIndex _output_get)
    (Audio|PlaySoundatLocation "/Game/Audio/SFX/SC_AxedHit.SC_AxedHit" (Transformation|GetActorLocation (Utilities|Array|Get(acopy) _output_get)) "0, 0, 0" 1.0 1.0 0.0 0 0 0)
    (for _array_element _output_get
      (Game|Damage|ApplyDamage _array_element (Variables|Default|GetWhack%20Damaged) (Pawn|GetController) self))
    (CallFunction|SetGateOpen true)
    (else
      (CallFunction|SetGateOpen true))))

(fn AlertStatusChangeNotifier
  (params (New%20State :type E_MinerStates%20Enum :default "NewEnumerator0"))
  (switch Utilities|FlowControl|Switch|SwitchonE_MinerStates New%20State
    (:NewEnumerator0
      (Default|CallAllClear (Utilities|GetDisplayName self)))
    (:NewEnumerator1
      (Default|CallOnAlert (Utilities|GetDisplayName self)))))

(fn StatusChangeVFX
  (params (New%20State :type E_MinerStates%20Enum :default "NewEnumerator0"))
  (Rendering|Components|Light|SetLightColor (Variables|Default|GetRectLight) (Utilities|Select :Index New%20State :NewEnumerator0 "(R=1.000000,G=0.672443,B=0.658375,A=1.000000)" :NewEnumerator1 "(R=1.000000,G=0.109375,B=0.159347,A=1.000000)") true))

(fn StatusChangeMovement
  (params (New%20State :type E_MinerStates%20Enum%20%28by%20ref%29 :default "NewEnumerator0"))
  (bind _output_get (Variables|/Script/Engine.CharacterMovementComponent|SetMaxWalkSpeed (Variables|Character|GetCharacterMovement) (.Value (Utilities|Map|Find (Variables|Default|GetSpeed) New%20State))))
  (Components|Timeline|SetPlayRate (Variables|/Script/ActorSequence.ActorSequenceComponent|GetSequencePlayer (Variables|Default|GetWalking)) (|(CurrentSpeed/PatrolSpeed) _output_get (.Value (Utilities|Map|Find (Variables|Default|GetSpeed) "")))))

(fn GetNextPatrolPoint
  (params (Current%20Point :type Actor%20Object%20Reference))
  (bind _astarget_point (Utilities|Casting|CastToTargetPoint Current%20Point)
    (:then
      (return (Utilities|Array|Get(acopy) (Variables|Default|GetPatrol%20Points) (Math|Integer|SelectInt 0 (+ (Utilities|Array|FindItem (Variables|Default|GetPatrol%20Points) _astarget_point) 1) (== (Utilities|Array|FindItem (Variables|Default|GetPatrol%20Points) _astarget_point) (Utilities|Array|LastIndex (Variables|Default|GetPatrol%20Points)))))))
    (:CastFailed
      (return (Utilities|Array|Get(acopy) (Variables|Default|GetPatrol%20Points))))))