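; Player character for a local multiplayer loot game: collects ore from chests, deposits it at delivery zones, and is coloured by controller ID.
; Timer-driven vacuuming sphere-traces and messages hit actors, snaps aim when idle, and steals ore from other players.
; Expel releases held physics objects or repeatedly shoots ore, with knockback through a brief Flying movement mode.
; Carried loot drives movement encumbrance, jiggle animation rate and a diegetic gold-and-text display.
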(event Collision|EventActorBeginOverlap
  (params (OtherActor :type Actor%20Object%20Reference))
  ;[1 1 1] Store Loot in container
  (Utilities|IsValid OtherActor
    (:Is%20Valid
      (if (Actor|ActorHasTag OtherActor "LootDelivery")
        (Class|BPILoot|ReceiveLoot(Message) OtherActor (Variables|Default|GetCurrent%20Loot))
        (CallFunction|UpdateLootAmount 0.0)))))

(event EventLoot
  (params (Amount :type Float%20%28single-precision%29))
  ;[1 1 1] Collect Loot from Chest
  (CallFunction|UpdateLootAmount (+ Amount (Variables|Default|GetCurrent%20Loot)))
  (Audio|PlaySoundatLocation (select (Utilities|Time|IsValidTimerHandle (Variables|Default|GetVacuuming%20Timer)) "/Game/Audio/SFX/SC_AbsorbedOre.SC_AbsorbedOre" "/Game/Audio/SFX/SC_GainedOre.SC_GainedOre") (Transformation|GetActorLocation) "0, 0, 0" 1.0 1.0 0.0 0 0 0))

(event Game|Damage|EventAnyDamage
  (params (Damage :type Float%20%28single-precision%29) (DamageType :type Damage%20Type%20Object%20Reference) (InstigatedBy :type Controller%20Object%20Reference) (DamageCauser :type Actor%20Object%20Reference))
  (Audio|PlaySoundatLocation "/Game/Audio/SFX/SC_AxeKilled.SC_AxeKilled" (Transformation|GetActorLocation) "0, 0, 0" 1.0 1.0 0.0 0 0 0)
  (Actor|DestroyActor))

(event EventTick
  (params (DeltaSeconds :type Float%20%28single-precision%29))
  (CallFunction|CharacterTurning)
  (CallFunction|UpdateWalkingAnimationPlaying))

(event EventVacuumed
  (params (Perpetrator :type Actor%20Object%20Reference))
  (if (and (Math|Float|NearlyEqual(Float) (Math|Vector|DotProduct (Transformation|GetActorForwardVector Perpetrator) (Math|Vector|NegateVector (Transformation|GetActorForwardVector))) -1.0 0.8) (!= (Variables|Default|GetCurrent%20Loot) 0.0))
    (Utilities|FlowControl|DoOnce false :!label _label
      (:Completed
        (Variables|Default|SetCurrent%20Loot (Math|Float|Clamp(Float) (- (Variables|Default|GetCurrent%20Loot) (Variables|Default|GetOre%20Stole%20Amount)) 0.0 (Variables|Default|GetMaximum%20Loot%20Carry)))
        (CallFunction|UpdateDiegeticOreDisplay)
        (Class|BPILoot|ReceiveLoot(Message) Perpetrator (Variables|Default|GetOre%20Stole%20Amount))
        (Utilities|FlowControl|Delay (Variables|Default|GetStole%20Frequency))
        (goto _label Reset)))))

(event EventPossessed
  (params (NewController :type Controller%20Object%20Reference))
  (CallFunction|UpdateColour))

(event Input|ActionEvents|InputActionInteract
  (params (Key :type Key%20Structure))
  ;[1 1 1] Collect Loot from Chest
  (:Pressed
    (if (< (Variables|Default|GetCurrent%20Loot) (Variables|Default|GetMaximum%20Loot%20Carry))
      (CallFunction|GetLoot)
      (bind _returnvalue (Utilities|Time|SetTimerbyFunctionName self "Get Loot" 0.48 true))
      (Variables|Default|SetLooting%20Timer _returnvalue)))
  (:Released
    (Utilities|Time|ClearandInvalidateTimerbyHandle (Variables|Default|GetLooting%20Timer))))

(event Input|ActionEvents|InputActionVacuum
  (params (Key :type Key%20Structure))
  (:Pressed
    (CallFunction|InitiateVacuuming))
  (:Released
    (CallFunction|TerminateVacuuming)))

(event Input|ActionEvents|InputActionExpel
  (params (Key :type Key%20Structure))
  (:Pressed
    (Utilities|IsValid (Class|PhysicsHandleComponent|GetGrabbedComponent (Variables|Default|GetPhysicsHandle))
      (:Is%20Valid
        (CallFunction|ExpelPhysicsObject))
      (:Is%20Not%20Valid
        (if (CallFunction|CanExpelOre)
          (bind _returnvalue (Utilities|Time|SetTimerbyFunctionName self "Expel Ore" (Variables|Default|GetExpel%20Ore%20Frequency) true))
          (Variables|Default|SetExpelling%20Ore%20Timer _returnvalue)
          (CallFunction|ExpelOre)
          (else
            (CallFunction|NoExpel))))))
  (:Released
    (Utilities|Time|ClearandInvalidateTimerbyHandle (Variables|Default|GetExpelling%20Ore%20Timer))))

(event Input|AxisEvents|InputAxisForward
  (params (AxisValue :type Float%20%28single-precision%29))
  (Pawn|Input|AddMovementInput "1.000000, 0, 0" AxisValue false))

(event Input|AxisEvents|InputAxisRight
  (params (AxisValue :type Float%20%28single-precision%29))
  (Pawn|Input|AddMovementInput "0.000000,1.000000, 0" AxisValue false))

(fn ConstructionScript
  (Rendering|SetVisibility (Variables|Default|GetGold) false true)
  (CallFunction|AdjustSpeedtoEncoumberement)
  (SplineMesh|SetEndPosition (Variables|Default|GetSplineMesh) (Math|Vector|MakeVector (Variables|Default|GetVacuum%20Range) 0.0 0.0) true)
  (CallFunction|InitMaterial))

(fn CharacterTurning
  (bind _returnvalue (Transformation|GetActorRotation))
  (bind _charactermovement (Variables|Character|GetCharacterMovement))
  (bind _velocity (Variables|/Script/Engine.MovementComponent|GetVelocity _charactermovement))
  (bind _returnvalue_2 (Math|Conversions|RotationFromXVector _velocity))
  (bind _returnvalue_3 (Math|Rotator|Delta(Rotator) _returnvalue_2 _returnvalue))
  ;[1 1 1] Is Moving
  (if (Math|Vector|NotEqual(Vector) (Class|Pawn|GetLastMovementInputVector) "0, 0, 0" 0.1)
    ;[1 1 1] Check angle
    (if (Utilities|Enum|NotEqual(Enum) _returnvalue_3 "0, 0, 0" (Variables|Default|GetTurn%20Speed))
      (Pawn|Input|AddControllerYawInput (* (.Yaw (Math|Rotator|BreakRotator _returnvalue_3)) (Variables|Default|GetTurn%20Speed) (Utilities|Time|GetWorldDeltaSeconds))))))

(fn UpdateLootAmount
  (params (Value :type Float%20%28single-precision%29))
  (Variables|Default|SetCurrent%20Loot (Math|Float|Clamp(Float) Value 0.0 (Variables|Default|GetMaximum%20Loot%20Carry)))
  (CallFunction|UpdateDiegeticOreDisplay))

(fn GetLoot
  (if (< (Variables|Default|GetCurrent%20Loot) (Variables|Default|GetMaximum%20Loot%20Carry))
    (for _array_element (Collision|GetOverlappingActors "/Game/Blueprints/Loot/BP_LootChest.BP_LootChest_C" :!class /Script/Engine.Actor)
      (Class|BPILoot|TryGettingLoot(Message) _array_element self))
    (else
      (Utilities|Time|ClearandInvalidateTimerbyHandle (Variables|Default|GetLooting%20Timer)))))

(fn Vacuuming
  (bind _vacuum_muzzle (Variables|Default|GetVacuum%20Muzzle))
  (if (CallFunction|CanVacuum)
    (if (Math|Vector|Equal(Vector) (Class|Pawn|GetLastMovementInputVector) "0, 0, 0" 0.1)
      (CallFunction|SnaptoVacuumingTarget))
    (bind _outhits (Collision|MultiSphereTraceForObjects (+ (Transformation|GetWorldLocation _vacuum_muzzle) (* (Math|Vector|GetForwardVector _vacuum_muzzle) (Variables|/Script/Engine.CapsuleComponent|GetCapsuleRadius (Variables|Collision|GetCapsuleComponent)))) (+ (Transformation|GetActorLocation) (* (Transformation|GetActorForwardVector) (Variables|Default|GetVacuum%20Range))) (Variables|Default|GetVacuum%20Radius) (Utilities|Array|MakeArray "ObjectTypeQuery2" "ObjectTypeQuery3" "ObjectTypeQuery4") false 0 "None" true "(R=1.000000,G=0.000000,B=0.000000,A=1.000000)" "(R=0.000000,G=1.000000,B=0.000000,A=1.000000)" 0.1))
    (for _array_element _outhits
      (Class|BPIVaccuumable|Vacuumed(Message) (.HitActor (Collision|BreakHitResult _array_element)) self))
    (else
      (CallFunction|TerminateVacuuming))))

(fn SnaptoVacuumingTarget
  (bind _vacuum_muzzle (Variables|Default|GetVacuum%20Muzzle))
  (bind (_outhit _returnvalue) (Class|KismetSystemLibrary|BoxTraceSingleforObjects (+ (Transformation|GetWorldLocation _vacuum_muzzle) (* (Math|Vector|GetForwardVector _vacuum_muzzle) (Variables|/Script/Engine.CapsuleComponent|GetCapsuleRadius (Variables|Collision|GetCapsuleComponent)))) (+ (Transformation|GetActorLocation) (* (Transformation|GetActorForwardVector) (Variables|Default|GetVacuum%20Range))) (Math|Vector|MakeVector 0.0 8e+01 (.OutHalfHeight (Components|Capsule|GetScaledCapsuleSize (Variables|Collision|GetCapsuleComponent)))) (Transformation|GetActorRotation) (Utilities|Array|MakeArray "ObjectTypeQuery2" "ObjectTypeQuery3" "ObjectTypeQuery4") false 0 "None" true))
  (if _returnvalue
    (Pawn|Input|AddControllerYawInput (/ (.yaw (Math|Rotator|Delta(Rotator) (Math|Rotator|FindLookatRotation (Transformation|GetActorLocation) (.ImpactPoint (Collision|BreakHitResult _outhit))) (Transformation|GetActorRotation))) 1e+01))))

(fn CanVacuum
  (return (and (< (Variables|Default|GetCurrent%20Loot) (Variables|Default|GetMaximum%20Loot%20Carry)) (not (Utilities|IsValid (Class|PhysicsHandleComponent|GetGrabbedComponent (Variables|Default|GetPhysicsHandle)))))))

(fn VacuumBlocked)

(fn NoExpel)

(fn ExpelPhysicsObject
  (Physics|Components|PhysicsHandle|ReleaseComponent (Variables|Default|GetPhysicsHandle)))

(fn ExpelOre
  (bind _vacuum_muzzle (Variables|Default|GetVacuum%20Muzzle))
  (bind _charactermovement (Variables|Character|GetCharacterMovement))
  (bind _returnvalue (Transformation|GetWorldTransform _vacuum_muzzle))
  (if (CallFunction|CanExpelOre)
    (Variables|Default|SetCurrent%20Loot (Math|Float|Clamp(Float) (- (Variables|Default|GetCurrent%20Loot) (Variables|Default|GetOre%20Shot%20Amount)) 0.0 (Variables|Default|GetMaximum%20Loot%20Carry)))
    (CallFunction|UpdateDiegeticOreDisplay)
    (Components|Movement|StopMovementImmediately _charactermovement)
    (Pawn|Components|CharacterMovement|SetMovementMode _charactermovement "MOVE_Flying" 0)
    (Sequencer|Player|Play (Variables|/Script/ActorSequence.ActorSequenceComponent|GetSequencePlayer (Variables|Default|GetExpulsion)) :!class /Script/MovieScene.MovieSceneSequencePlayer)
    (Audio|Components|Audio|Play (Variables|Default|GetExpel%20Audio) 0.0)
    (Game|SpawnActorfromClass "/Game/Blueprints/Loot/BP_GoldOre.BP_GoldOre_C" (Math|Transform|MakeTransform (+ (.location _returnvalue) (* (Math|Vector|GetForwardVector (.rotation _returnvalue)) 6e+01)) (Transformation|GetActorRotation) (* "1.000000,1.000000,-1.000000" (Math|Random|RandomFloatinRange 0.5 0.7))) "Undefined" 0 (Math|Random|RandomFloatinRange 6.8e+02 9.2e+02) 0)
    (Physics|AddImpulse (Variables|Character|GetCharacterMovement) (* (Math|Vector|NegateVector (Transformation|GetActorForwardVector)) (Variables|Default|GetOre%20Shot%20Knockback%20Impulse)) true)
    (Utilities|Time|SetTimerbyFunctionName self "Stop Floating" (Variables|Default|GetOre%20Shot%20Knockback%20Duration))
    (else
      (Utilities|Time|ClearandInvalidateTimerbyHandle (Variables|Default|GetExpelling%20Ore%20Timer)))))

(fn UpdateDiegeticOreDisplay
  (bind _current_loot (Variables|Default|GetCurrent%20Loot))
  (bind _maximum_loot_carry (Variables|Default|GetMaximum%20Loot%20Carry))
  (bind _returnvalue (/ _current_loot _maximum_loot_carry))
  ;[1 1 1] Textual Counter Update
  (Rendering|Components|TextRender|SetText (Variables|Default|GetTextRender) (Utilities|Text|FormatText "{value}/{max}" (Variables|Default|GetCurrent%20Loot) (Variables|Default|GetMaximum%20Loot%20Carry)))
  (CallFunction|AdjustSpeedtoEncoumberement)
  (Rendering|SetVisibility (Variables|Default|GetGold) false true)
  (if (== (Variables|Default|GetCurrent%20Loot) (Variables|Default|GetMaximum%20Loot%20Carry))
    (Rendering|SetVisibility (Variables|Default|GetGold) true true)
    (elif (>= _returnvalue 0.75)
      (Rendering|SetVisibility (Variables|Default|GetGold1) true true)
      (elif (>= _returnvalue 0.5)
        (Rendering|SetVisibility (Variables|Default|GetGold2) true true)
        (elif (>= _returnvalue 0.25)
          (Rendering|SetVisibility (Variables|Default|GetGold3) true true)
          (elif (!= (Variables|Default|GetCurrent%20Loot) 0.0)
            (Rendering|SetVisibility (Variables|Default|GetGold4) true false)))))))

(fn CanExpelOre
  (return (or (!= (Variables|Default|GetCurrent%20Loot) 0.0) (and (Class|LowEntryExtendedStandardLibrary|WithEditor) (Variables|Default|GetInfinity%20Ore%20Bullets)))))

(fn AdjustSpeedtoEncoumberement
  (Variables|/Script/Engine.CharacterMovementComponent|SetMaxWalkSpeed (Variables|Character|GetCharacterMovement) (- (.Value (Utilities|Map|Find (Variables|Default|GetDefault%20Movement%20Metrics) "Max Walk Speed")) (* (Variables|Default|GetCurrent%20Loot) 1e+01)))
  (Variables|/Script/Engine.CharacterMovementComponent|SetMaxAcceleration (Variables|Character|GetCharacterMovement) (- (.Value (Utilities|Map|Find (Variables|Default|GetDefault%20Movement%20Metrics) "Max Acceleration")) (* (Variables|Default|GetCurrent%20Loot) 1.2)))
  (Variables|/Script/Engine.CharacterMovementComponent|SetBrakingDecelerationWalking (Variables|Character|GetCharacterMovement) (|(Default-((ML-CL)*60)) (.Value (Utilities|Map|Find (Variables|Default|GetDefault%20Movement%20Metrics) "Braking Deceleration Walking")) (Variables|Default|GetCurrent%20Loot) (Variables|Default|GetMaximum%20Loot%20Carry)))
  (bind _sequenceplayer (Variables|/Script/ActorSequence.ActorSequenceComponent|GetSequencePlayer (Variables|Default|GetWalking%20Jiggle))
    (:then
      (Components|Timeline|SetPlayRate _sequenceplayer (Math|Float|MapRangeClamped (Variables|/Script/Engine.CharacterMovementComponent|GetMaxWalkSpeed (Variables|Character|GetCharacterMovement)) 3e+02 6e+02 1.0 2.5)))
    (:else)))

(fn StopFloating
  (bind _charactermovement (Variables|Character|GetCharacterMovement))
  (switch Utilities|FlowControl|Switch|SwitchonEMovementMode (Variables|/Script/Engine.CharacterMovementComponent|GetMovementMode (Variables|Character|GetCharacterMovement))
    (:MOVE_Flying
      (Pawn|Components|CharacterMovement|SetMovementMode _charactermovement "MOVE_Walking" 0)
      (Components|Movement|StopMovementImmediately _charactermovement))))

(fn TerminateVacuuming
  (bind _default_movement_metrics (Variables|Default|GetDefault%20Movement%20Metrics))
  (Utilities|Time|ClearandInvalidateTimerbyHandle (Variables|Default|GetVacuuming%20Timer))
  (|SetBy-RefVar (.Value (Utilities|Map|Find _default_movement_metrics "Max Walk Speed")) (.Value (Utilities|Map|Find _default_movement_metrics "Walk Speed Default")))
  (CallFunction|AdjustSpeedtoEncoumberement)
  (Class|MovieSceneSequencePlayer|GotoEndandStop (Variables|/Script/ActorSequence.ActorSequenceComponent|GetSequencePlayer (Variables|Default|GetVacuum%20Jiggle)))
  (Development|SetHiddeninGame (Variables|Default|GetSplineMesh) true false)
  (Audio|Components|Audio|FadeOut (Variables|Default|GetVacuum%20Audio) 0.62 0.0 :!class /Script/Engine.AudioComponent))

(fn InitiateVacuuming
  (if (CallFunction|CanVacuum)
    (CallFunction|AdjustSpeedtoEncoumberement)
    (CallFunction|Vacuuming)
    (bind _returnvalue (Utilities|Time|SetTimerbyFunctionName self "Vacuuming" 0.1 true))
    (Variables|Default|SetVacuuming%20Timer _returnvalue)
    (Class|MovieSceneSequencePlayer|PlayLooping (Variables|/Script/ActorSequence.ActorSequenceComponent|GetSequencePlayer (Variables|Default|GetVacuum%20Jiggle)) -1)
    (Development|SetHiddeninGame (Variables|Default|GetSplineMesh) false false)
    (Audio|Components|Audio|FadeIn (Variables|Default|GetVacuum%20Audio) 0.08 1.0 0.0 :!class /Script/Engine.AudioComponent)))

(fn UpdateWalkingAnimationPlaying
  (if (Math|Vector|NotEqual(Vector) (Class|Pawn|GetLastMovementInputVector) "0, 0, 0" 0.1)
    (if (not (Audio|Components|Audio|IsPlaying (Variables|/Script/ActorSequence.ActorSequenceComponent|GetSequencePlayer (Variables|Default|GetWalking%20Jiggle))))
      (Class|MovieSceneSequencePlayer|PlayLooping (Variables|/Script/ActorSequence.ActorSequenceComponent|GetSequencePlayer (Variables|Default|GetWalking%20Jiggle)) -1))
    (elif (Audio|Components|Audio|IsPlaying (Variables|/Script/ActorSequence.ActorSequenceComponent|GetSequencePlayer (Variables|Default|GetWalking%20Jiggle)))
      (Class|MovieSceneSequencePlayer|GotoEndandStop (Variables|/Script/ActorSequence.ActorSequenceComponent|GetSequencePlayer (Variables|Default|GetWalking%20Jiggle))))))

(fn InitMaterial
  (bind _returnvalue (Rendering|Material|CreateDynamicMaterialInstance (Variables|Default|GetBackpack) 0 "/Game/Materials/MI_Backpack.MI_Backpack" "None" :!class /Script/Engine.PrimitiveComponent))
  (bind _output_get (Variables|Default|SetPlayer%20Colour%20Mat _returnvalue))
  (Rendering|Material|SetMaterial (Variables|Default|GetFacet) 1 _output_get)
  (Rendering|Material|SetMaterial (Variables|Default|GetBackpack) 0 (Variables|Default|GetPlayer%20Colour%20Mat)))

(fn UpdateColour
  (bind _asplayer_controller (Utilities|Casting|CastToPlayerController (Pawn|GetController)))
  (Rendering|Material|SetVectorParameterValue (Variables|Default|GetPlayer%20Colour%20Mat) "Colour" (Utilities|Select :Index (Class|GameplayStatics|GetPlayerControllerID _asplayer_controller) :Option%200 "(R=1.000000,G=0.829889,B=0.263283,A=1.000000)" :Option%201 "(R=0.000000,G=0.569136,B=1.000000,A=1.000000)" :Option%202 "(R=1.000000,G=0.000000,B=0.047706,A=1.000000)" :Option%203 "(R=0.000000,G=1.000000,B=0.020782,A=1.000000)") :!class /Script/Engine.MaterialInstanceDynamic))