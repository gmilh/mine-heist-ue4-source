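; Player controller for local or multiplayer play that handles joining, respawning and quitting.
; The first key press without a valid pawn deploys, once only, the BPI_Lift actor whose index matches the controller ID.
; When a possessed pawn is destroyed, it restarts the player after a short delay at the start spot GM_Multiplayer_Base assigns.
; Holding Pause for about two seconds quits the game through a timer that release cancels.
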(event `InputAction|Pause`
  (params (Key :type "Key Structure"))
  (:`Pressed`
    (bind _returnvalue (`KismetSystemLibrary.K2_SetTimerDelegate` (delegate `Quit`) 2.1)))
  (:`Released`
    (`KismetSystemLibrary.K2_ClearAndInvalidateTimerHandle` _returnvalue)))

(event `Quit`
  (`KismetSystemLibrary.QuitGame` null "Quit"))

(event `self.ReceivePossess`
  (params (PossessedPawn :type "Pawn Object Reference"))
  (add `self.OnDestroyed` PossessedPawn (delegate `Handle Pawn Destruction`)))

(event `Handle Pawn Destruction` :!signature `self.OnDestroyed`
  (params (DestroyedActor :type "Actor Object Reference"))
  (bind _returnvalue (`GameplayStatics.GetGameMode`))
  (`KismetSystemLibrary.Delay` 0.2)
  (bind _asgm_multiplayer_base (cast `/Game/Blueprints/GameMode/GM_Multiplayer_Base` _returnvalue))
  (`GameModeBase.RestartPlayerAtPlayerStart` _returnvalue self (`/Game/Blueprints/GameMode/GM_Multiplayer_Base.Get Start Spot by Player Index` _asgm_multiplayer_base self)))

(event `Key|AnyKey` :consume false :overrideparent false
  (params (Key :type "Key Structure"))
  (:`Pressed`
    (`/Engine/EditorBlueprintResources/StandardMacros.IsValid` (`self.K2_GetPawn`)
      (:`Is Not Valid`
        (`/Engine/EditorBlueprintResources/StandardMacros.DoOnce` false
          (:`Completed`
            (bind _outactors (`GameplayStatics.GetAllActorsWithInterface` "/Game/Blueprints/GameMode/BPI_Lift.BPI_Lift_C"))
            (for _array_element _outactors
              (bind _player_index (message `/Game/Blueprints/GameMode/BPI_Lift.Check Index` _array_element))
              (if (== _player_index (`GameplayStatics.GetPlayerControllerID` self))
                (message `/Game/Blueprints/GameMode/BPI_Lift.Deploy Lift` _array_element)
                (break)))))))))

(fn `UserConstructionScript`)